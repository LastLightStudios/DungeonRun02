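; Base grid-battle unit that takes its mesh, anim class, attack and health from a DT_Units row and is driven by BP_UnitController with BT_Unit.
; It finds the nearest enemy in MyGrid and steps one orthogonal square along the longer axis, trying the other axis if blocked.
; Attacks go through EquippedWeapon; damage and healing functions update a widget health bar, and death removes the unit from the grid.
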(event Custom|OnDeath
  (Default|DestroyUnit (Variables|Default|GetMyGrid) self)
  (Actor|DestroyActor)
  (Development|PrintString (Utilities|String|Append (Utilities|GetDisplayName self) " has died!")))

(event EventBeginPlay
  (CallFunction|SetStats)
  (Variables|/Game/Blueprints/Unit/WGT_Health_Bar.WGT_Health_Bar_C|SetTeam (Combat|GetHealthBar) (Variables|Stats|GetTeam)))

(event Collision|EventActorBeginOverlap
  (params (OtherActor :type Actor%20Object%20Reference)))

(event EventTick
  (params (DeltaSeconds :type Float%20%28single-precision%29)))

(event EventHeal
  (params (Incoming%20Heal :type Float%20%28single-precision%29)))

(event EventDamage
  (params (Incoming%20Damage :type Float%20%28single-precision%29))
  (bind _post_mitigation_damage (Combat|CalculateDamageTaken Incoming%20Damage))
  (Combat|TakeDamage _post_mitigation_damage))

(fn ConstructionScript
  (CallFunction|SetupCosmetics)
  (Variables|Default|SetAIControllerClass "/Game/Blueprints/AI/BP_UnitController.BP_UnitController_C"))

(fn SetFocus
  (params (IsFocused :type Boolean))
  (if IsFocused
    (Rendering|SetRenderCustomDepth (Variables|Character|GetMesh) true)
    (Rendering|SetCustomDepthStencilValue (Variables|Character|GetMesh) 251)
    (else
      (Rendering|SetRenderCustomDepth (Variables|Character|GetMesh) false))))

(fn SetMovingState
  (params (IsBeingMoved :type Boolean))
  (Handling|SetMeshRelativeZState IsBeingMoved))

(fn SetMeshRelativeZState
  (params (Is%20Being%20Moved :type Boolean))
  (if Is%20Being%20Moved
    (Variables|Default|SetIsBeingMoved true)
    (Transformation|AddLocalOffset (Variables|Character|GetMesh) (Math|Vector|MakeVector 0.0 0.0 (LocalVariables|GetZ%20Offset)) false false)
    (else
      (Variables|Default|SetIsBeingMoved false)
      (Transformation|AddLocalOffset (Variables|Character|GetMesh) (Math|Vector|MakeVector 0.0 0.0 (* -1 (LocalVariables|GetZ%20Offset))) false false))))

(fn SetupCosmetics
  (bind _mesh (Variables|Character|GetMesh))
  (bind _returnvalue (Utilities|GetDataTableRow "/Game/Data/DT_Units.DT_Units" (.RowName (Utilities|Struct|BreakDataTableRowHandle (Variables|Stats|GetUnit%20Row))))
    (:then
      (Class|SkinnedMeshComponent|SetSkeletalMesh _mesh (.Mesh (Utilities|Struct|BreakFUnit _returnvalue)) true)
      (Class|SkeletalMeshComponent|SetAnimClass _mesh (.ABP (Utilities|Struct|BreakFUnit _returnvalue))))))

(fn RunBT
  (AI|RunBehaviorTree (AI|GetAIController self) "/Game/Blueprints/AI/BT_Unit.BT_Unit"))

(fn FindNearestEnemy
  (bind _self self)
  (bind _returnvalue (Transformation|GetActorLocation _self))
  (LocalVariables|SetClosest%20Enemy 0)
  (for _array_element (Variables|/Game/Blueprints/Level/BP_Grid.BP_Grid_C|GetUnits (Variables|Default|GetMyGrid))
    (if (and (Utilities|Enum|NotEqual(Enum) (Variables|Stats|GetTeam) (Variables|BP_Unit_C|GetTeam _array_element)) (Utilities|Enum|NotEqual(Enum) (Variables|BP_Unit_C|GetTeam _array_element) "NewEnumerator2"))
      ;[1 1 1] Verify there is a Closest Enemy
      (Utilities|IsValid (LocalVariables|GetClosest%20Enemy)
        (:Is%20Valid
          (if (<= (Math|Vector|Distance(Vector) (Transformation|GetActorLocation _array_element) _returnvalue) (Math|Vector|Distance(Vector) _returnvalue (Transformation|GetActorLocation (LocalVariables|GetClosest%20Enemy))))
            (LocalVariables|SetClosest%20Enemy _array_element :!label _label)))
        (:Is%20Not%20Valid
          (goto _label)))))
  (return (LocalVariables|GetClosest%20Enemy)))

(fn FindNextMove
  (params (Target%20Square :type BP%20Square%20Object%20Reference))
  (LocalVariables|SetTarget%20X (Variables|/Game/Blueprints/Level/BP_Square.BP_Square_C|GetX%20Location Target%20Square))
  (LocalVariables|SetTarget%20Y (Variables|/Game/Blueprints/Level/BP_Square.BP_Square_C|GetY%20Location Target%20Square))
  (Utilities|FlowControl|Sequence
    (:then_0
      ;[1 1 1] Sees if already atop the Target
      (if (and (== (- (Variables|Default|GetX%20Location) (LocalVariables|GetTarget%20X)) 0) (== (- (Variables|Default|GetY%20Location) (LocalVariables|GetTarget%20Y)) 0))
        (Development|PrintString "Already atop the target location")
        ;[1 1 1] Should return square unit is on
        (bind _found_square (Default|FindSquare (Variables|Default|GetMyGrid) (Variables|Default|GetX%20Location) (Variables|Default|GetY%20Location)))
        (return _found_square)
        (else
          (Utilities|FlowControl|Sequence
            (:then_0
              (Math|Integer|CompareInt (- (Variables|Default|GetX%20Location) (LocalVariables|GetTarget%20X))
                (:>
                  ;[1 1 1] CASE: Set Temp X in direction of Target X
                  (LocalVariables|SetTemp%20X (- (Variables|Default|GetX%20Location) 1)))
                (:==
                  ;[1 1 1] CASE: This Unit and Target Unit are in the same X
                  (LocalVariables|SetTemp%20X (Variables|Default|GetX%20Location)))
                (:<
                  (LocalVariables|SetTemp%20X (+ (Variables|Default|GetX%20Location) 1)))))
            (:then_1
              (Math|Integer|CompareInt (- (Variables|Default|GetY%20Location) (LocalVariables|GetTarget%20Y))
                (:>
                  ;[1 1 1] CASE: Set Temp Y in direction of Target Y
                  (LocalVariables|SetTemp%20Y (- (Variables|Default|GetY%20Location) 1)))
                (:==
                  ;[1 1 1] CASE: This Unit and Target Unit are in the same Y
                  (LocalVariables|SetTemp%20Y (Variables|Default|GetY%20Location)))
                (:<
                  (LocalVariables|SetTemp%20Y (+ (Variables|Default|GetY%20Location) 1)))))))))
    (:then_1
      ;[1 1 1] Try to move in the direction that is furthest away
      (Math|Integer|CompareInt (Math|Integer|Absolute(Integer) (- (Variables|Default|GetX%20Location) (LocalVariables|GetTarget%20X))) (Math|Integer|Absolute(Integer) (- (Variables|Default|GetY%20Location) (LocalVariables|GetTarget%20Y)))
        (:>
          (bind _found_unit (Default|FindUnit (Variables|Default|GetMyGrid) (LocalVariables|GetTemp%20X) (Variables|Default|GetY%20Location)))
          (Utilities|IsValid _found_unit
            (:Is%20Valid
              (bind _found_unit_2 (Default|FindUnit (Variables|Default|GetMyGrid) (Variables|Default|GetX%20Location) (LocalVariables|GetTemp%20Y)))
              (Utilities|IsValid _found_unit_2
                (:Is%20Valid
                  ;[1 1 1] CASE: Occupied, so stay still
                  (LocalVariables|SetNext%20X (Variables|Default|GetX%20Location))
                  (LocalVariables|SetNext%20Y (Variables|Default|GetY%20Location)))
                (:Is%20Not%20Valid
                  ;[1 1 1] CASE: Unoccupied Square, so Set as Next
                  (LocalVariables|SetNext%20X (Variables|Default|GetX%20Location))
                  (LocalVariables|SetNext%20Y (LocalVariables|GetTemp%20Y)))))
            (:Is%20Not%20Valid
              ;[1 1 1] CASE: Unoccupied Square, so Set as Next
              (LocalVariables|SetNext%20X (LocalVariables|GetTemp%20X))
              (LocalVariables|SetNext%20Y (Variables|Default|GetY%20Location)))))
        (:==
          (bind _found_unit_3 (Default|FindUnit (Variables|Default|GetMyGrid) (Variables|Default|GetX%20Location) (LocalVariables|GetTemp%20Y) :!label _label))
          (Utilities|IsValid _found_unit_3
            (:Is%20Valid
              (bind _found_unit_4 (Default|FindUnit (Variables|Default|GetMyGrid) (LocalVariables|GetTemp%20X) (Variables|Default|GetY%20Location)))
              (Utilities|IsValid _found_unit_4
                (:Is%20Valid
                  ;[1 1 1] CASE: Occupied, so stay still
                  (LocalVariables|SetNext%20X (Variables|Default|GetX%20Location))
                  (LocalVariables|SetNext%20Y (Variables|Default|GetY%20Location)))
                (:Is%20Not%20Valid
                  ;[1 1 1] CASE: Unoccupied Square, so Set as Next
                  (LocalVariables|SetNext%20X (LocalVariables|GetTemp%20X))
                  (LocalVariables|SetNext%20Y (Variables|Default|GetY%20Location)))))
            (:Is%20Not%20Valid
              ;[1 1 1] CASE: Unoccupied Square, so Set as Next
              (LocalVariables|SetNext%20X (Variables|Default|GetX%20Location))
              (LocalVariables|SetNext%20Y (LocalVariables|GetTemp%20Y)))))
        (:<
          (goto _label))))
    (:then_2
      (bind _found_square_2 (Default|FindSquare (Variables|Default|GetMyGrid) (LocalVariables|GetNext%20X) (LocalVariables|GetNext%20Y)))
      (return _found_square_2))))

(fn SetStats
  (bind _returnvalue (Utilities|GetDataTableRow "/Game/Data/DT_Units.DT_Units" (.RowName (Utilities|Struct|BreakDataTableRowHandle (Variables|Stats|GetUnit%20Row))))
    (:then
      (Variables|Stats|SetAttack%20Value (.AttackValue (Utilities|Struct|BreakFUnitStats (.UnitStats (Utilities|Struct|BreakFUnit _returnvalue)))))
      (bind _output_get (Variables|Stats|SetMaximum%20Health (.MaximumHealthPoints (Utilities|Struct|BreakFUnitStats (.UnitStats (Utilities|Struct|BreakFUnit _returnvalue))))))
      (bind _output_get_2 (Variables|Stats|SetCurrent%20Health _output_get))
      (Default|SetMaximumHealth (Combat|GetHealthBar) _output_get_2))))

(fn GetHealthBar
  (Utilities|IsValid (Variables|UI|GetHealth%20Bar%20Ref)
    (:Is%20Valid
      _)
    (:Is%20Not%20Valid
      (bind _aswgt_health_bar (Utilities|Casting|CastToWGT_Health_Bar (UserInterface|GetUserWidgetObject (Variables|Default|GetWGC_Health_Bar))))
      (Variables|UI|SetHealth%20Bar%20Ref _aswgt_health_bar)))
  (return (Variables|UI|GetHealth%20Bar%20Ref)))

(fn CalculateDamageTaken
  (params (Pre-Mitigation%20Damage :type Float%20%28single-precision%29))
  (return Pre-Mitigation%20Damage))

(fn TakeDamage
  (params (Incoming%20Damage :type Float%20%28single-precision%29))
  (bind _output_get (Variables|Stats|SetCurrent%20Health (- (Variables|Stats|GetCurrent%20Health) Incoming%20Damage)))
  (if (<= _output_get 0.0)
    (Default|SetCurrentHealth (Combat|GetHealthBar) 0.0)
    (CallFunction|OnDeath)
    (else
      (Default|SetCurrentHealth (Combat|GetHealthBar) _output_get))))

(fn RecoverHealth
  (params (Incoming%20Heal :type Float%20%28single-precision%29))
  (bind _output_get (Variables|Stats|SetCurrent%20Health (+ Incoming%20Heal (Variables|Stats|GetCurrent%20Health))))
  (if (>= _output_get (Variables|Stats|GetMaximum%20Health))
    (bind _output_get_2 (Variables|Stats|SetCurrent%20Health (Variables|Stats|GetMaximum%20Health)))
    (Default|SetCurrentHealth (Combat|GetHealthBar) _output_get_2)
    (else
      (Default|SetCurrentHealth (Combat|GetHealthBar) (Variables|Stats|GetCurrent%20Health)))))

(fn BasicAttack
  (params (TargetEnemy :type BP%20Unit%20Object%20Reference))
  (Development|PrintString (Utilities|String|Append (Utilities|GetDisplayName self) " is attacking" (Utilities|GetDisplayName TargetEnemy)))
  (Default|BasicAttackAction (Variables|Default|GetEquipped%20Weapon) self TargetEnemy))