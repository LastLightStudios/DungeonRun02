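; Weapon component that gives a unit a generic melee basic attack on a square grid.
; BasicAttack sends the target damage equal to the owner unit's attack value plus the owning BP_Weapon's.
; FindValidSquaresToAttackFrom scans the 3x3 block around the enemy, collecting squares without units and flagging whether the attacker is already there.
; FindTargetSquareInAttackRange returns the attacker's current square if in range, otherwise the nearest valid one by 2D distance.
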(event EventBeginPlay
  (|CallParentFunction) ; This node is disabled and will not be called.\nDrag off pins to build functionality.
)

(event EventTick
  (params (DeltaSeconds :type Float%20%28single-precision%29))
  (|CallParentFunction DeltaSeconds) ; This node is disabled and will not be called.\nDrag off pins to build functionality.
)

(event EventBasicAttack
  (params (Owner%20Unit :type BP%20Unit%20Object%20Reference) (Target%20Enemy :type BP%20Unit%20Object%20Reference))
  (bind _asbp_weapon (Utilities|Casting|CastToBP_Weapon (Components|GetOwner)))
  (Class|BPIDamagable|ReceiveDamage(Message) Target%20Enemy (+ (Variables|/Game/Blueprints/Unit/BP_Unit.BP_Unit_C|GetAttack%20Value Owner%20Unit) (Variables|/Game/Blueprints/Weapon/BP_Weapon.BP_Weapon_C|GetAttackValue _asbp_weapon))))

(fn FindTargetSquareinAttackRange
  (params (Owner%20Unit :type BP%20Unit%20Object%20Reference) (Target%20Enemy :type BP%20Unit%20Object%20Reference))
  (bind _output_get (LocalVariables|Set_OwnerUnit Owner%20Unit))
  (bind (_valid_squares _isinrange) (CallFunction|FindValidSquarestoAttackfrom _output_get Target%20Enemy))
  (if _isinrange
    (bind _found_square (Default|FindSquare (Variables|/Game/Blueprints/Unit/BP_Unit.BP_Unit_C|GetMyGrid (LocalVariables|Get_OwnerUnit)) (Variables|/Game/Blueprints/Unit/BP_Unit.BP_Unit_C|GetX%20Location (LocalVariables|Get_OwnerUnit)) (Variables|/Game/Blueprints/Unit/BP_Unit.BP_Unit_C|GetY%20Location (LocalVariables|Get_OwnerUnit))))
    (LocalVariables|Set_TargetSquare _found_square)
    (else
      (for _array_element _valid_squares
        (Utilities|IsValid (LocalVariables|Get_TargetSquare)
          (:Is%20Valid
            (Math|Float|CompareFloat (Math|Vector|Distance2D(Vector) (Transformation|GetActorLocation _array_element) (Transformation|GetActorLocation (LocalVariables|Get_OwnerUnit))) (Math|Vector|Distance2D(Vector) (Transformation|GetActorLocation (LocalVariables|Get_TargetSquare)) (Transformation|GetActorLocation (LocalVariables|Get_OwnerUnit)))
              (:<
                (LocalVariables|Set_TargetSquare _array_element))))
          (:Is%20Not%20Valid
            (LocalVariables|Set_TargetSquare _array_element))))))
  (return (LocalVariables|Get_TargetSquare)))

(fn FindValidSquarestoAttackfrom
  (params (Owner%20Unit :type BP%20Unit%20Object%20Reference) (Target%20Enemy :type BP%20Unit%20Object%20Reference))
  (LocalVariables|Set_OwnerUnit Owner%20Unit)
  (LocalVariables|Set_TargetEnemy Target%20Enemy)
  (LocalVariables|Set_IsInRange false)
  (Utilities|FlowControl|Sequence
    (:then_0
      (LocalVariables|SetEnemy%20X (Variables|/Game/Blueprints/Unit/BP_Unit.BP_Unit_C|GetX%20Location (LocalVariables|Get_TargetEnemy)))
      (LocalVariables|SetEnemy%20Y (Variables|/Game/Blueprints/Unit/BP_Unit.BP_Unit_C|GetY%20Location (LocalVariables|Get_TargetEnemy))))
    (:then_1
      (for _index (range (- (LocalVariables|GetEnemy%20X) 1) (+ (LocalVariables|GetEnemy%20X) 1))
        (for _index_2 (range (- (LocalVariables|GetEnemy%20Y) 1) (+ (LocalVariables|GetEnemy%20Y) 1))
          (bind _found_unit (Default|FindUnit (Variables|/Game/Blueprints/Unit/BP_Unit.BP_Unit_C|GetMyGrid (LocalVariables|Get_TargetEnemy)) _index _index_2))
          (Utilities|IsValid _found_unit
            (:Is%20Valid
              (if (== (LocalVariables|Get_OwnerUnit) _found_unit)
                (LocalVariables|Set_IsInRange true)))
            (:Is%20Not%20Valid
              (bind _found_square (Default|FindSquare (Variables|/Game/Blueprints/Unit/BP_Unit.BP_Unit_C|GetMyGrid (LocalVariables|Get_TargetEnemy)) _index _index_2))
              (Utilities|Array|AddUnique (LocalVariables|Get_ValidSquares) _found_square)))))
      (return (LocalVariables|Get_ValidSquares) (LocalVariables|Get_IsInRange)))))