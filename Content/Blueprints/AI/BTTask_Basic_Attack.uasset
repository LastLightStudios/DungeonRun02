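; Behavior tree task that makes an AI-controlled BP_Unit perform a basic attack on its blackboard enemy.
; On AI execute, it casts the controlled pawn and the GetEnemy blackboard object to BP_Unit and stores them as Owner and Enemy.
; It then calls BasicAttack on the owner with that enemy and immediately finishes, always reporting failure to the tree.
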(event EventReceiveExecuteAI
  (params (OwnerController :type AI%20Controller%20Object%20Reference) (ControlledPawn :type Pawn%20Object%20Reference))
  (Utilities|FlowControl|Sequence
    (:then_0
      (bind _asbp_unit (Utilities|Casting|CastToBP_Unit ControlledPawn))
      (Variables|Default|SetOwner _asbp_unit)
      (bind _asbp_unit_2 (Utilities|Casting|CastToBP_Unit (Class|BTFunctionLibrary|GetBlackboardValueasObject (Variables|Default|GetGet%20Enemy))))
      (Variables|Default|SetEnemy _asbp_unit_2))
    (:then_1
      (Default|BasicAttack (Variables|Default|GetOwner) (Variables|Default|GetEnemy))
      (AI|BehaviorTree|FinishExecute false))))