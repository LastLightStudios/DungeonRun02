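; Behavior tree task that picks the next grid square for a BP_Unit on the way to its target.
; It reads the target BP_Square from the blackboard, asks the unit's FindNextMove for the next square and stores that in the next-location key.
; It then copies that square's X and Y grid coordinates onto the unit and finishes with success, without moving the pawn itself.
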(event EventReceiveExecuteAI
  (params (OwnerController :type AI%20Controller%20Object%20Reference) (ControlledPawn :type Pawn%20Object%20Reference))
  (bind _asbp_unit (Utilities|Casting|CastToBP_Unit ControlledPawn))
  (Utilities|FlowControl|Sequence
    (:then_0
      (bind _asbp_square (Utilities|Casting|CastToBP_Square (Class|BTFunctionLibrary|GetBlackboardValueasObject (Variables|Default|GetGet%20Target%20Location))))
      (bind _next_location (Default|FindNextMove _asbp_unit _asbp_square))
      (Class|BTFunctionLibrary|SetBlackboardValueasObject (Variables|Default|GetSet%20Next%20Location) _next_location))
    (:then_1
      (Variables|/Game/Blueprints/Unit/BP_Unit.BP_Unit_C|SetX%20Location _asbp_unit (Variables|/Game/Blueprints/Level/BP_Square.BP_Square_C|GetX%20Location _next_location))
      (Variables|/Game/Blueprints/Unit/BP_Unit.BP_Unit_C|SetY%20Location _asbp_unit (Variables|/Game/Blueprints/Level/BP_Square.BP_Square_C|GetY%20Location _next_location))
      (AI|BehaviorTree|FinishExecute true))))