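; Player controller for mouse drag-and-drop placement of units on a square grid.
; Each tick it traces the cursor location, sphere-traces there to highlight the BP_Square beneath, and drags any held unit along.
; Releasing left mouse moves or swaps a picked-up unit via Grid, or returns it when off-grid.
; Newly created units follow the cursor until release, joining an empty square or being destroyed otherwise.
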(event Custom|Created%20Unit
  (params (Created%20Unit :type BP%20Unit%20Object%20Reference))
  (Variables|Default|SetNew%20Unit%20Created true)
  (bind _output_get (Variables|Default|SetMoving%20Unit Created%20Unit))
  (Default|SetFocus _output_get true)
  (Default|SetMovingState _output_get true))

(event EventBeginPlay
  (bind _asbp_new_game_mode (Utilities|Casting|CastToBP_NewGameMode (Game|GetGameMode)))
  (Variables|Default|SetGameMode _asbp_new_game_mode))

(event EventTick
  (params (DeltaSeconds :type Float%20%28single-precision%29))
  (Variables|Default|SetCursor%20Location (CallFunction|FindCursorLocation))
  (Focus|FindFocusedSquare)
  (Moving|SelectedUnitFollowsCursor))

(event Input|ActionEvents|InputActionExitGame
  (params (Key :type Key%20Structure :default "None"))
  (:Pressed
    (Development|ExecuteConsoleCommand "Exit" 0)))

(event Input|MouseEvents|LeftMouseButton
  (params (Key :type Key%20Structure :default "None"))
  (:Pressed
    (Utilities|IsValid (Focus|GetUnitinFocusedSquare)
      (:Is%20Valid
        (Moving|StartMovingUnit))))
  (:Released
    (if (Variables|Default|GetIs%20Moving%20Unit)
      (Moving|StopMovingUnit)
      (elif (Variables|Default|GetNew%20Unit%20Created)
        (CallFunction|StopMovingCreatedUnit)))))

(event Input|KeyboardEvents|Z
  (params (Key :type Key%20Structure :default "None"))
  (:Pressed
    (for _array_element (Variables|/Game/Blueprints/Level/BP_Grid.BP_Grid_C|GetUnits (Variables|Default|GetGrid))
      (Development|PrintString (Utilities|String|Append (Utilities|GetDisplayName _array_element) ": " (Utilities|String|ToString(Integer) (Variables|/Game/Blueprints/Unit/BP_Unit.BP_Unit_C|GetX%20Location _array_element)) ", " (Utilities|String|ToString(Integer) (Variables|/Game/Blueprints/Unit/BP_Unit.BP_Unit_C|GetY%20Location _array_element)) " Wielding " (Variables|/Game/Blueprints/Weapon/BP_Weapon.BP_Weapon_C|GetDisplayName (Variables|/Game/Blueprints/Unit/BP_Unit.BP_Unit_C|GetEquipped%20Weapon _array_element)))))))

(fn ConstructionScript)

(fn FindCursorLocation
  (return (.Location (Collision|BreakHitResult (.HitResult (Game|Player|GetHitResultUnderCursorbyChannel "TraceTypeQuery4" true))))))

(fn FindFocusedSquare
  (bind _cursor_location (Variables|Default|GetCursor%20Location))
  (bind _outhits (Collision|MultiSphereTraceByChannel _cursor_location (+ _cursor_location "0, 0,1.000000") 1.0 "TraceTypeQuery3" false 0 "None"))
  (if (> (Utilities|Array|Length _outhits) 0)
    (Utilities|IsValid (.HitActor (Collision|BreakHitResult (Utilities|Array|Get(acopy) _outhits)))
      (:Is%20Valid
        (bind _asbp_square (Utilities|Casting|CastToBP_Square (.HitActor (Collision|BreakHitResult (Utilities|Array|Get(acopy) _outhits))))
          (:then
            (if (!= _asbp_square (Variables|Default|GetFocused%20Square))
              (Focus|UnfocusSquare)
              (Focus|SetFocusedSquare _asbp_square)))
          (:CastFailed
            (Focus|UnfocusSquare :!label _label)
            (Variables|Default|SetFocused%20Square 0))))
      (:Is%20Not%20Valid
        (goto _label)))
    (else
      (goto _label))))

(fn UnfocusSquare
  (Utilities|IsValid (Variables|Default|GetFocused%20Square)
    (:Is%20Valid
      (if (== (Variables|Default|GetOriginal%20Position) (Variables|Default|GetFocused%20Square))
        (Default|SetFocus (Variables|Default|GetOriginal%20Position) 2)
        (else
          (Default|SetFocus (Variables|Default|GetFocused%20Square)))))))

(fn GetUnitinFocusedSquare
  (bind _focused_square (Variables|Default|GetFocused%20Square))
  (Utilities|IsValid (Variables|Default|GetFocused%20Square)
    (:Is%20Valid
      (bind _found_unit (Default|FindUnit (Variables|Default|GetGrid) (Variables|/Game/Blueprints/Level/BP_Square.BP_Square_C|GetX%20Location _focused_square) (Variables|/Game/Blueprints/Level/BP_Square.BP_Square_C|GetY%20Location _focused_square)))
      (LocalVariables|SetNewLocalVar_0 _found_unit))
    (:Is%20Not%20Valid
      _))
  (return (LocalVariables|GetNewLocalVar_0)))

(fn SetFocusedSquare
  (params (In%20Square :type BP%20Square%20Object%20Reference))
  (bind _output_get (Variables|Default|SetFocused%20Square In%20Square))
  (Default|SetFocus _output_get 1))

(fn StartMovingUnit
  (Variables|Default|SetIs%20Moving%20Unit true)
  (Variables|Default|SetOriginal%20Position (Variables|Default|GetFocused%20Square))
  (bind _output_get (Variables|Default|SetMoving%20Unit (Focus|GetUnitinFocusedSquare)))
  (Default|SetMovingState _output_get true)
  (Default|SetFocus _output_get true))

(fn StopMovingUnit
  (bind _focused_square (Variables|Default|GetFocused%20Square))
  (Default|SetMovingState (Variables|Default|GetMoving%20Unit) false)
  (Default|SetFocus (Variables|Default|GetMoving%20Unit) false)
  (Utilities|IsValid (Variables|Default|GetOriginal%20Position)
    (:Is%20Valid
      (Default|SetFocus (Variables|Default|GetOriginal%20Position))
      (Utilities|IsValid (Variables|Default|GetFocused%20Square)
        (:Is%20Valid
          ;[1 1 1] Is Hovered Location Occupied?
          (bind _found_unit (Default|FindUnit (Variables|Default|GetGrid) (Variables|/Game/Blueprints/Level/BP_Square.BP_Square_C|GetX%20Location _focused_square) (Variables|/Game/Blueprints/Level/BP_Square.BP_Square_C|GetY%20Location _focused_square)))
          (bind _output_get (LocalVariables|SetSecond%20Unit _found_unit))
          (Utilities|IsValid _output_get
            (:Is%20Valid
              ;[1 1 1] CASE: Swap Unit with Occupied Square
              (Default|SwapUnits (Variables|Default|GetGrid) (Variables|Default|GetMoving%20Unit) (LocalVariables|GetSecond%20Unit))
              (Utilities|MoveUnitLocationtoSquare (Variables|Default|GetMoving%20Unit) (Variables|Default|GetFocused%20Square)
                (:Exec%20Out
                  (Utilities|MoveUnitLocationtoSquare (LocalVariables|GetSecond%20Unit) (Variables|Default|GetOriginal%20Position)
                    (:Exec%20Out
                      _)))))
            (:Is%20Not%20Valid
              ;[1 1 1] CASE: Move to Empty Square
              (Default|MoveUnit (Variables|Default|GetGrid) (Variables|Default|GetMoving%20Unit) (Variables|Default|GetFocused%20Square))
              (Utilities|MoveUnitLocationtoSquare (Variables|Default|GetMoving%20Unit) (Variables|Default|GetFocused%20Square)
                (:Exec%20Out
                  _)))))
        (:Is%20Not%20Valid
          ;[1 1 1] CASE: Hovering Invalid Location
          (Default|MoveUnit (Variables|Default|GetGrid) (Variables|Default|GetMoving%20Unit) (Variables|Default|GetOriginal%20Position))
          (Utilities|MoveUnitLocationtoSquare (Variables|Default|GetMoving%20Unit) (Variables|Default|GetOriginal%20Position)
            (:Exec%20Out
              _))))
      (Variables|Default|SetMoving%20Unit 0)
      (Variables|Default|SetOriginal%20Position 0)
      (Variables|Default|SetIs%20Moving%20Unit false))))

(fn SelectedUnitFollowsCursor
  (bind _cursor_location (Variables|Default|GetCursor%20Location))
  (Utilities|IsValid (Variables|Default|GetMoving%20Unit)
    (:Is%20Valid
      (Transformation|SetActorLocation (Variables|Default|GetMoving%20Unit) (Math|Vector|MakeVector (.x _cursor_location) (.y _cursor_location) (.z (Transformation|GetActorLocation (Variables|Default|GetMoving%20Unit)))) false false))))

(fn StopMovingCreatedUnit
  (bind _focused_square (Variables|Default|GetFocused%20Square))
  (Utilities|IsValid (Variables|Default|GetFocused%20Square)
    (:Is%20Valid
      (Utilities|FlowControl|Sequence
        (:then_0
          (Default|SetMovingState (Variables|Default|GetMoving%20Unit) false)
          (Default|SetFocus (Variables|Default|GetMoving%20Unit) false))
        (:then_1
          (bind _found_unit (Default|FindUnit (Variables|Default|GetGrid) (Variables|/Game/Blueprints/Level/BP_Square.BP_Square_C|GetX%20Location _focused_square) (Variables|/Game/Blueprints/Level/BP_Square.BP_Square_C|GetY%20Location _focused_square)))
          (Utilities|IsValid _found_unit
            (:Is%20Valid
              (Actor|DestroyActor (Variables|Default|GetMoving%20Unit)))
            (:Is%20Not%20Valid
              (Default|AddUnittoGrid (Variables|Default|GetGrid) (Variables|Default|GetMoving%20Unit) (Variables|Default|GetFocused%20Square))
              (Utilities|MoveUnitLocationtoSquare (Variables|Default|GetMoving%20Unit) (Variables|Default|GetFocused%20Square)
                (:Exec%20Out
                  _))))
          (Variables|Default|SetNew%20Unit%20Created false :!label _label)
          (Variables|Default|SetMoving%20Unit 0))))
    (:Is%20Not%20Valid
      (Actor|DestroyActor (Variables|Default|GetMoving%20Unit))
      (goto _label))))