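; Tile-based combat board that tracks squares and units and decides when a fight ends.
; Construction spawns BP_Square child actors; InitGrid registers placed BP_Units, deriving tile coordinates from their world positions.
; Lookups scan flat arrays by coordinate, while move and swap edit only unit coordinates, not transforms.
; LoadEnemyGrid spawns enemies, StartCombat runs unit behavior trees, and DestroyUnit reports the winner to BP_NewGameMode once either team is empty.
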(event Custom|Init%20Grid
  (bind _asbp_new_game_mode (Utilities|Casting|CastToBP_NewGameMode (Game|GetGameMode)))
  (Variables|Default|SetGameMode _asbp_new_game_mode)
  (CallFunction|TempAssignUnits)
  (bind _outactors (Actor|GetAllActorsOfClass "/Game/Blueprints/Unit/BP_Unit.BP_Unit_C"))
  (for _array_element _outactors
    (Variables|/Game/Blueprints/Unit/BP_Unit.BP_Unit_C|SetMyGrid _array_element self)
    (Development|PrintString (Utilities|String|Append (Utilities|GetDisplayName _array_element) " at:" (Utilities|String|ToString(Integer) (Variables|/Game/Blueprints/Unit/BP_Unit.BP_Unit_C|GetX%20Location _array_element)) ", " (Utilities|String|ToString(Integer) (Variables|/Game/Blueprints/Unit/BP_Unit.BP_Unit_C|GetY%20Location _array_element))))))

(event Custom|DestroyUnit
  (params (DeadUnit :type BP%20Unit%20Object%20Reference))
  (Utilities|Array|RemoveItem (Variables|Default|GetUnits) DeadUnit)
  (bind (_combatends _winner) (CallFunction|CheckifCombatEnd))
  (if _combatends
    (Default|CombatEnd (Variables|Default|GetGameMode) _winner)))

(event EventBeginPlay)

(event Collision|EventActorBeginOverlap
  (params (OtherActor :type Actor%20Object%20Reference)))

(event EventTick
  (params (DeltaSeconds :type Float%20%28single-precision%29)))

(fn ConstructionScript
  (CallFunction|BuildGrid))

(fn BuildGrid
  (bind _gridsize (Variables|Default|GetGridSize))
  (bind _squareclass (Variables|Default|GetSquareClass))
  (bind _squareclass_2 (Variables|Default|GetSquareClass))
  (bind (_x _y) (Math|Vector2D|BreakVector2D _gridsize))
  (bind _tile_size (Utilities|GetClassDefaults _squareclass))
  (bind _tile_size_2 (Utilities|GetClassDefaults _squareclass_2))
  (bind _returnvalue (/ _tile_size 2.0))
  (for _index (range 0 (- (Math|Float|Truncate _x) 1))
    (LocalVariables|SetX _index)
    (for _index_2 (range 0 (- (Math|Float|Truncate _y) 1))
      (LocalVariables|SetY _index_2)
      (bind _returnvalue_2 (AddComponent|AddChildActorComponent false (Math|Transform|MakeTransform (Math|Vector|MakeVector (+ (* (LocalVariables|GetX) _tile_size_2) _returnvalue) (+ (* (LocalVariables|GetY) _tile_size_2) _returnvalue) 0.0))))
      (bind _asbp_square (Utilities|Casting|CastToBP_Square (Variables|/Script/Engine.ChildActorComponent|GetChildActor _returnvalue_2)))
      (Utilities|Array|AddUnique (Variables|Default|GetSquares) _asbp_square)
      (Variables|/Game/Blueprints/Level/BP_Square.BP_Square_C|SetX%20Location _asbp_square (LocalVariables|GetX))
      (Variables|/Game/Blueprints/Level/BP_Square.BP_Square_C|SetY%20Location _asbp_square (LocalVariables|GetY)))))

(fn TempAssignUnits
  (bind _squareclass (Variables|Default|GetSquareClass))
  (bind _tile_size (Utilities|GetClassDefaults _squareclass))
  (bind _outactors (Actor|GetAllActorsOfClass "/Game/Blueprints/Unit/BP_Unit.BP_Unit_C"))
  (for _array_element _outactors
    (Utilities|Array|Add (Variables|Default|GetUnits) _array_element)
    (Variables|/Game/Blueprints/Unit/BP_Unit.BP_Unit_C|SetX%20Location _array_element (Math|Float|Floor (.x (/ (- (Transformation|GetActorLocation _array_element) (Transformation|GetActorLocation)) (Math|Vector|MakeVector _tile_size _tile_size 1.0)))))
    (Variables|/Game/Blueprints/Unit/BP_Unit.BP_Unit_C|SetY%20Location _array_element (Math|Float|Floor (.y (/ (- (Transformation|GetActorLocation _array_element) (Transformation|GetActorLocation)) (Math|Vector|MakeVector _tile_size _tile_size 1.0)))))))

(fn AddUnittoGrid
  (params (In%20Unit :type BP%20Unit%20Object%20Reference) (Destination%20Square :type BP%20Square%20Object%20Reference))
  (bind _returnvalue (Utilities|Array|AddUnique (Variables|Default|GetUnits) In%20Unit))
  (if (== _returnvalue -1)
    (Development|PrintString "Already exists")
    (else
      (Variables|/Game/Blueprints/Unit/BP_Unit.BP_Unit_C|SetX%20Location In%20Unit (Variables|/Game/Blueprints/Level/BP_Square.BP_Square_C|GetX%20Location Destination%20Square))
      (Variables|/Game/Blueprints/Unit/BP_Unit.BP_Unit_C|SetY%20Location In%20Unit (Variables|/Game/Blueprints/Level/BP_Square.BP_Square_C|GetY%20Location Destination%20Square))
      (Variables|/Game/Blueprints/Unit/BP_Unit.BP_Unit_C|SetMyGrid In%20Unit self))))

(fn MoveUnit
  (params (Unit :type BP%20Unit%20Object%20Reference) (Destination%20Square :type BP%20Square%20Object%20Reference))
  (LocalVariables|SetIn%20Unit Unit)
  (LocalVariables|SetDestination%20X (Variables|/Game/Blueprints/Level/BP_Square.BP_Square_C|GetX%20Location Destination%20Square))
  (LocalVariables|SetDestination%20Y (Variables|/Game/Blueprints/Level/BP_Square.BP_Square_C|GetY%20Location Destination%20Square))
  (bind _found_unit (CallFunction|FindUnit (LocalVariables|GetDestination%20X) (LocalVariables|GetDestination%20Y)))
  (Utilities|IsValid _found_unit
    (:Is%20Valid
      (Development|PrintString "ERROR: Destination Occupied"))
    (:Is%20Not%20Valid
      (Variables|/Game/Blueprints/Unit/BP_Unit.BP_Unit_C|SetX%20Location (LocalVariables|GetIn%20Unit) (LocalVariables|GetDestination%20X))
      (Variables|/Game/Blueprints/Unit/BP_Unit.BP_Unit_C|SetY%20Location (LocalVariables|GetIn%20Unit) (LocalVariables|GetDestination%20Y))))
  (return))

(fn SwapUnits
  (params (Origin%20Unit :type BP%20Unit%20Object%20Reference) (Destination%20Unit :type BP%20Unit%20Object%20Reference))
  (LocalVariables|SetFirst%20Unit Origin%20Unit)
  (LocalVariables|SetSecond%20Unit Destination%20Unit)
  (Utilities|FlowControl|Sequence
    (:then_0
      (LocalVariables|SetOrigin%20X (Variables|/Game/Blueprints/Unit/BP_Unit.BP_Unit_C|GetX%20Location (LocalVariables|GetFirst%20Unit)))
      (LocalVariables|SetOrigin%20Y (Variables|/Game/Blueprints/Unit/BP_Unit.BP_Unit_C|GetY%20Location (LocalVariables|GetFirst%20Unit))))
    (:then_1
      (Variables|/Game/Blueprints/Unit/BP_Unit.BP_Unit_C|SetX%20Location (LocalVariables|GetFirst%20Unit) (Variables|/Game/Blueprints/Unit/BP_Unit.BP_Unit_C|GetX%20Location (LocalVariables|GetSecond%20Unit)))
      (Variables|/Game/Blueprints/Unit/BP_Unit.BP_Unit_C|SetY%20Location (LocalVariables|GetFirst%20Unit) (Variables|/Game/Blueprints/Unit/BP_Unit.BP_Unit_C|GetY%20Location (LocalVariables|GetSecond%20Unit))))
    (:then_2
      (Variables|/Game/Blueprints/Unit/BP_Unit.BP_Unit_C|SetX%20Location (LocalVariables|GetSecond%20Unit) (LocalVariables|GetOrigin%20X))
      (Variables|/Game/Blueprints/Unit/BP_Unit.BP_Unit_C|SetY%20Location (LocalVariables|GetSecond%20Unit) (LocalVariables|GetOrigin%20Y)))))

(fn FindUnit
  (params (X%20Location :type Integer) (Y%20Location :type Integer))
  (LocalVariables|SetOut%20Unit 0)
  (for _array_element (Variables|Default|GetUnits)
    (if (and (== X%20Location (Variables|/Game/Blueprints/Unit/BP_Unit.BP_Unit_C|GetX%20Location _array_element)) (== Y%20Location (Variables|/Game/Blueprints/Unit/BP_Unit.BP_Unit_C|GetY%20Location _array_element)))
      (bind _output_get (LocalVariables|SetOut%20Unit _array_element))
      (return _output_get))))

(fn FindSquare
  (params (X%20Location :type Integer) (Y%20Location :type Integer))
  (LocalVariables|SetOut%20Square 0)
  (for _array_element (Variables|Default|GetSquares)
    (if (and (== X%20Location (Variables|/Game/Blueprints/Level/BP_Square.BP_Square_C|GetX%20Location _array_element)) (== Y%20Location (Variables|/Game/Blueprints/Level/BP_Square.BP_Square_C|GetY%20Location _array_element)))
      (bind _output_get (LocalVariables|SetOut%20Square _array_element))
      (return _output_get))))

(fn LoadEnemyGrid
  (params (EnemyUnits :type Array%20of%20BP%20Unit%20Object%20References))
  (bind _squareclass (Variables|Default|GetSquareClass))
  (bind _squareclass_2 (Variables|Default|GetSquareClass))
  (bind _tile_size (Utilities|GetClassDefaults _squareclass))
  (bind _tile_size_2 (Utilities|GetClassDefaults _squareclass_2))
  (bind _returnvalue (/ _tile_size 2.0))
  (for _array_element EnemyUnits
    (bind _output_get (LocalVariables|SetCurrent%20Unit _array_element))
    (Game|SpawnActorfromClass "/Game/Blueprints/Unit/BP_Unit.BP_Unit_C" (Math|Transform|MakeTransform (Math|Vector|MakeVector (+ (* (Variables|/Game/Blueprints/Unit/BP_Unit.BP_Unit_C|GetX%20Location (LocalVariables|GetCurrent%20Unit)) _tile_size_2) _returnvalue) (+ (* (Variables|/Game/Blueprints/Unit/BP_Unit.BP_Unit_C|GetY%20Location (LocalVariables|GetCurrent%20Unit)) _tile_size_2) _returnvalue) 0.0)) "Undefined" 0 (Variables|/Game/Blueprints/Unit/BP_Unit.BP_Unit_C|GetUnit%20Row _output_get) "NewEnumerator1" 0)))

(fn StartCombat
  (for _array_element (Variables|Default|GetUnits)
    (Default|RunBT _array_element)))

(fn CheckifCombatEnd
  (Utilities|FlowControl|Sequence
    (:then_0
      (LocalVariables|SetNumberOfPlayerUnits 0)
      (LocalVariables|SetNumberofEnemyUnits 0)
      (LocalVariables|SetisCombatEnding false)
      (LocalVariables|SetNewLocalVar_0 "NewEnumerator2"))
    (:then_1
      (for _array_element (Variables|Default|GetUnits)
        (switch Utilities|FlowControl|Switch|SwitchonETeam (Variables|/Game/Blueprints/Unit/BP_Unit.BP_Unit_C|GetTeam _array_element)
          (:NewEnumerator0
            (Math|Integer|IncrementInt (LocalVariables|GetNumberOfPlayerUnits)))
          (:NewEnumerator1
            (Math|Integer|IncrementInt (LocalVariables|GetNumberofEnemyUnits)))))
      (if (== (LocalVariables|GetNumberOfPlayerUnits) 0)
        (Development|PrintString "player lost")
        (LocalVariables|SetisCombatEnding true)
        (LocalVariables|SetNewLocalVar_0 "NewEnumerator1")
        (elif (== (LocalVariables|GetNumberofEnemyUnits) 0)
          (Development|PrintString "Player Won")
          (LocalVariables|SetisCombatEnding true)
          (LocalVariables|SetNewLocalVar_0 "NewEnumerator0"))))
    (:then_2
      (return (LocalVariables|GetisCombatEnding) (LocalVariables|GetNewLocalVar_0)))))