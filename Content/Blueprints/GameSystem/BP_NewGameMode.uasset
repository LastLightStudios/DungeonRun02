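; BP_NewGameMode is a game mode that tracks the game phase and handles the end of combat.
; On BeginPlay it sets the initial phase, caches BP_GameInstance and binds its return-to-main-menu dispatcher to open the MainMenu level.
; CombatEnd shows a WGT_PostCombatScreen for the given victor team, then switches the phase.
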(event Custom|CombatEnd
  (params (CombatVictor :type ETeam%20Enum :default "NewEnumerator0"))
  (bind _returnvalue (UserInterface|CreateWidget "/Game/Blueprints/Widget/WGT_PostCombatScreen.WGT_PostCombatScreen_C"))
  (Variables|/Game/Blueprints/Widget/WGT_PostCombatScreen.WGT_PostCombatScreen_C|SetTeam _returnvalue CombatVictor)
  (UserInterface|Viewport|AddtoPlayerScreen _returnvalue)
  (Variables|Default|SetGamePhase "NewEnumerator4"))

(event Custom|OnReturnToMainMenu
  (Game|OpenLevel(byName) "MainMenu"))

(event EventBeginPlay
  (Variables|Default|SetGamePhase "NewEnumerator0")
  (bind _asbp_game_instance (Utilities|Casting|CastToBP_GameInstance (Game|GetGameInstance)))
  (bind _output_get (Variables|Default|SetGameInstance _asbp_game_instance))
  (EventDispatchers|BindEventtoReturntoMainMenuDispatcher _output_get (delegate Custom|OnReturnToMainMenu)))

(event EventTick
  (params (DeltaSeconds :type Float%20%28single-precision%29)))

(fn ConstructionScript)